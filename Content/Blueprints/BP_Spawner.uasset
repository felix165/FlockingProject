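; BP_Spawner populates an area with BP_FlockChar actors and holds a shared RandomLocation, likely as the flock's target.
; From BeginPlay, a delayed loop spawns characters until SpawnedChar reaches SpawnCount.
; Each spawn uses random navmesh-reachable X/Y near the spawner at its height, retries on failure, receives a spawner reference and yaws toward the spawner.
; NewTargetLoc rerolls RandomLocation within a wider radius; SpawnCone is an empty stub.
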(event `self.ReceiveBeginPlay`
  (if (< (`KismetArrayLibrary.Array_Length` (`self.SpawnedChar`)) (`self.SpawnCount`)) :!label _label
    (`KismetSystemLibrary.Delay` 0.2)
    (`self.SpawnFlockChar`)
    (goto _label)))

(event `self.ReceiveTick`
  (params (DeltaSeconds :type "Float (single-precision)")))

(event `SpawnFlockChar`
  (bind _spawnedchar (`self.SpawnedChar`))
  (bind _randomlocation (`NavigationSystemV1.K2_GetRandomReachablePointInRadius` (`self.K2_GetActorLocation`) 500.0 null null))
  (bind _defaultsceneroot (`self.DefaultSceneRoot`))
  (bind (_returnvalue_x _returnvalue_y _returnvalue_z) (`KismetMathLibrary.BreakVector` (`SceneComponent.K2_GetComponentLocation` _defaultsceneroot)))
  (bind _returnvalue (`|SpawnActorFromClass` "/Game/Blueprints/BP_FlockChar.BP_FlockChar_C" (`KismetMathLibrary.MakeTransform` (`KismetMathLibrary.MakeVector` (.x _randomlocation) (.y _randomlocation) _returnvalue_z)) "Undefined" "OverrideRootScale" null self null :!label _label_2))
  (`/Engine/EditorBlueprintResources/StandardMacros.IsValid` _returnvalue
    (:`Is Valid`
      (bind _capsulecomponent (`Character.CapsuleComponent` _returnvalue))
      (bind (_returnvalue_roll _returnvalue_pitch _returnvalue_yaw) (`KismetMathLibrary.BreakRotator` (`KismetMathLibrary.Conv_VectorToRotator` (- (`SceneComponent.K2_GetComponentLocation` _defaultsceneroot) (`SceneComponent.K2_GetComponentLocation` _capsulecomponent)))))
      (`SceneComponent.K2_AddLocalRotation` _capsulecomponent (`KismetMathLibrary.MakeRotator` 0.0 0.0 _returnvalue_yaw) false false)
      (`KismetArrayLibrary.Array_Add` _spawnedchar _returnvalue)
      (`KismetSystemLibrary.PrintString` (`KismetStringLibrary.Conv_IntToString` (`KismetArrayLibrary.Array_Length` _spawnedchar))))
    (:`Is Not Valid`
      (goto _label_2))))

(event `NewTargetLoc`
  (bind _randomlocation (`NavigationSystemV1.K2_GetRandomReachablePointInRadius` (`self.K2_GetActorLocation`) 2000.0 null null))
  (bind (_returnvalue_x _returnvalue_y _returnvalue_z) (`KismetMathLibrary.BreakVector` (`SceneComponent.K2_GetComponentLocation` (`self.DefaultSceneRoot`))))
  (set `self.RandomLocation` (`KismetMathLibrary.MakeVector` (.x _randomlocation) (.y _randomlocation) _returnvalue_z)))

(fn `SpawnCone`)

(fn `UserConstructionScript`)